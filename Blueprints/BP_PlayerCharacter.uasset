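; First-person player character Blueprint that teleports to an aimed spot on left mouse click.
; Every Tick it line-traces in segments along a gravity-curved parabola from the camera, drawn with debug lines.
; A hit on a sufficiently upward-facing surface stores the target, enables teleporting and draws a debug cylinder there.
; Clicking moves the actor to that target, raised by the capsule half-height.
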(event EventBeginPlay)

(event Collision|EventActorBeginOverlap
  (params (OtherActor :type Actor%20Object%20Reference)))

(event EventTick
  (params (DeltaSeconds :type Float%20%28single-precision%29))
  (bind _firstpersoncameracomponent (Variables|Default|GetFirstPersonCameraComponent))
  (CallFunction|GetTeleportLocationParabola (Transformation|GetWorldLocation _firstpersoncameracomponent) (Math|Vector|GetForwardVector _firstpersoncameracomponent) 10 0.1 1.5e+03))

(event Input|MouseEvents|LeftMouseButton
  (params (Key :type Key%20Structure))
  (:Pressed
    (if (Variables|Default|GetbCanTeleport)
      (CallFunction|TeleporttoLocation (Variables|Default|GetTeleportLocation))
      (Development|PrintString "Teleport good"))))

(fn ConstructionScript)

(fn TeleporttoLocation
  (params (Location :type Vector))
  (Transformation|SetActorLocation (Math|Vector|MakeVector (.x Location) (.y Location) (+ (.z Location) (Variables|/Script/Engine.CapsuleComponent|GetCapsuleHalfHeight (Variables|Default|GetCapsuleComponent)))) false false))

(fn GetTeleportLocationParabola
  (params (Location :type Vector) (Forward :type Vector) (Steps :type Integer) (TimeStep :type Float%20%28single-precision%29) (Speed :type Float%20%28single-precision%29))
  (Utilities|FlowControl|Sequence
    (:then_0
      (bind _output_get (LocalVariables|SetInitialLocation Location))
      (LocalVariables|SetPreviousLocation _output_get)
      (LocalVariables|SetVelocity (* Forward Speed))
      (LocalVariables|SetTime TimeStep))
    (:then_1
      (bind _index (Utilities|FlowControl|ForLoopwithBreak 1 Steps :!label _label)
        (:LoopBody
          ;[1 1 1] missing interactive, teleport
          (bind (_outhit _returnvalue) (Collision|LineTraceByChannel (LocalVariables|GetPreviousLocation) (+ (Math|Vector|MakeVector (* (.X (Math|Vector|BreakVector (LocalVariables|GetVelocity))) (* _index (LocalVariables|GetTime))) (* (.Y (Math|Vector|BreakVector (LocalVariables|GetVelocity))) (* _index (LocalVariables|GetTime))) (- (* (.Z (Math|Vector|BreakVector (LocalVariables|GetVelocity))) (* _index (LocalVariables|GetTime))) (* (* _index (LocalVariables|GetTime)) (* _index (LocalVariables|GetTime)) 0.5 2e+03))) (LocalVariables|GetInitialLocation)) "TraceTypeQuery3" false 0 "ForOneFrame" true "(R=1.000000,G=0.009645,B=0.000000,A=1.000000)"))
          (LocalVariables|SetPreviousLocation (+ (Math|Vector|MakeVector (* (.X (Math|Vector|BreakVector (LocalVariables|GetVelocity))) (* _index (LocalVariables|GetTime))) (* (.Y (Math|Vector|BreakVector (LocalVariables|GetVelocity))) (* _index (LocalVariables|GetTime))) (- (* (.Z (Math|Vector|BreakVector (LocalVariables|GetVelocity))) (* _index (LocalVariables|GetTime))) (* (* _index (LocalVariables|GetTime)) (* _index (LocalVariables|GetTime)) 0.5 2e+03))) (LocalVariables|GetInitialLocation)))
          (if _returnvalue
            (Utilities|FlowControl|Sequence
              (:then_0
                (goto _label Break))
              (:then_1
                (if (> (Math|Vector|DotProduct (.Normal (Collision|BreakHitResult _outhit)) "0, 0,1.000000") 0.1)
                  (bind _output_get_2 (Variables|Default|SetbCanTeleport (> (Math|Vector|DotProduct (.Normal (Collision|BreakHitResult _outhit)) "0, 0,1.000000") 0.1)))
                  (if _output_get_2
                    (bind _output_get_3 (Variables|Default|SetTeleportLocation (.Location (Collision|BreakHitResult _outhit))))
                    (Class|KismetSystemLibrary|DrawDebugCylinder _output_get_3 (+ _output_get_3 (* (.Normal (Collision|BreakHitResult _outhit)) 1e+01)) 3e+01 25 "(R=0.000000,G=0.542093,B=1.000000,A=1.000000)" 0.0 1.0)))))
            (else
              (Variables|Default|SetbCanTeleport false))))))))