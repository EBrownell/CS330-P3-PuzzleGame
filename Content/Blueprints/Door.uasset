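; Door actor that stays shut with a key-needed message until its Open event sets CanOpen.
; Interact then plays a creaking sound and runs the DoorOpen timeline, which slides the mesh along its relative Y axis.
; The timeline update clears CanOpen, so later interactions print the key message again unless Open is called again.
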(event Custom|Open
  (Variables|Default|SetCan%20Open true))

(event EventBeginPlay)

(event Collision|EventActorBeginOverlap
  (params (OtherActor :type Actor%20Object%20Reference)))

(event EventTick
  (params (DeltaSeconds :type Float%20%28single-precision%29)))

(event EventInteract
  (bind _mesh (Variables|Default|GetMesh))
  (bind _relativelocation (Variables|/Script/Engine.SceneComponent|GetRelativeLocation _mesh))
  (if (Variables|Default|GetCan%20Open)
    (Audio|PlaySoundatLocation "/Game/Audio/Door_Creaking_Open.Door_Creaking_Open" (Transformation|GetWorldLocation (Variables|Default|GetMesh)) "0, 0, 0" 0.4 1.4 0.0 0 0 0)
    (bind _newtrack_3 (Timeline|Door%20Open Play)
      (:Update
        (Transformation|SetRelativeLocation _mesh (Math|Vector|MakeVector (.x _relativelocation) _newtrack_3 (.z _relativelocation)) false false)
        (Variables|Default|SetCan%20Open false)))
    (else
      (Development|PrintString "You need a key for me to open :)"))))

(fn ConstructionScript)