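; First-person player character that interacts with, carries, throws and uses objects, sprints, and can teleport by pointing.
; E traces from the camera to call Interactable actors or grab BPI_PickUps actors with a PhysicsHandle, which follows HeldObjectLocation each Tick.
; Left click triggers a held item's BPI_HeldAction; Q throws it with an impulse.
; T toggles teleport mode, where segmented traces along a gravity arc mark upward-facing landing spots that E teleports to.
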(event Custom|AttemptInteract
  (bind _firstpersoncameracomponent (Variables|Default|GetFirstPersonCameraComponent))
  (bind _returnvalue (Transformation|GetWorldLocation _firstpersoncameracomponent))
  ;[1 1 1] LineTrace to find Interactable / Simulates Physics (and Interact / Pickup)
  (bind (_outhit _returnvalue_2) (Collision|LineTraceByChannel _returnvalue (+ _returnvalue (* (Math|Vector|GetForwardVector _firstpersoncameracomponent) 400)) "TraceTypeQuery1" false 0 "None"))
  (if _returnvalue_2
    (bind _asinteractable (Utilities|Casting|CastToInteractable (.hitactor _outhit))
      (:then
        (Class|Interactable|Interact _asinteractable))
      (:CastFailed
        (if (Utilities|DoesObjectImplementInterface (.hitactor _outhit) "/Game/Final_level/BPI_PickUps.BPI_PickUps_C")
          (bind _asbpi_pick_ups (Utilities|Casting|CastToBPI_PickUps (.hitactor _outhit))
            (:then
              (Class|BPIPickUps|RemovePlayerCollision(Message) (Utilities|ToObject(Interface) _asbpi_pick_ups))
              (Variables|Default|SetHeldObjectActor (.hitactor _outhit))
              (bind _output_get (Variables|Default|SetHeldObject (.hitcomponent _outhit)))
              (Physics|Components|PhysicsHandle|GrabComponentatLocationwithRotation (Variables|Default|GetPhysicsHandle) (Variables|Default|GetHeldObject) "None" (.location (Transformation|GetWorldTransform _output_get)) (.rotation (Transformation|GetWorldTransform _output_get)))
              (Variables|Default|SetbIsHoldingObject true))
            (:CastFailed
              (Development|PrintString "Cast Failed (Char Pickup)"))))))))

(event Custom|DropObject
  ;[1 1 1] Drop Object in hand (if holding something)
  (if (Variables|Default|GetbIsHoldingObject)
    (Variables|Default|SetbIsHoldingObject false)
    (Physics|Components|PhysicsHandle|ReleaseComponent (Variables|Default|GetPhysicsHandle))
    (bind _asbpi_pick_ups (Utilities|Casting|CastToBPI_PickUps (Variables|Default|GetHeldObjectActor))
      (:then
        (Class|BPIPickUps|AddPlayerCollision(Message) (Utilities|ToObject(Interface) _asbpi_pick_ups)))
      (:CastFailed
        (Development|PrintString "Failed Cast")))))

(event Custom|PickUpObject
  (bind _firstpersoncameracomponent (Variables|Default|GetFirstPersonCameraComponent))
  (bind _returnvalue (Transformation|GetWorldLocation _firstpersoncameracomponent))
  ;[1 1 1] Pick Up Object
  (bind (_outhit _returnvalue_2) (Collision|LineTraceByChannel _returnvalue (+ _returnvalue (* (Math|Vector|GetForwardVector _firstpersoncameracomponent) 3e+02)) "TraceTypeQuery1" false 0 "None"))
  (if _returnvalue_2
    (if (Physics|IsSimulatingPhysics (.HitComponent (Collision|BreakHitResult _outhit)) "None")
      (bind _output_get (Variables|Default|SetHeldObject (.HitComponent (Collision|BreakHitResult _outhit))))
      (Transformation|SetWorldRotation (Variables|Default|GetHeldObjectLocation) (.rotation (Transformation|GetWorldTransform _output_get)) false false)
      (Physics|Components|PhysicsHandle|GrabComponentatLocationwithRotation (Variables|Default|GetPhysicsHandle) (Variables|Default|GetHeldObject) "None" (.location (Transformation|GetWorldTransform _output_get)) (.rotation (Transformation|GetWorldTransform _output_get)))
      (Collision|SetCollisionResponsetoChannel (Variables|Default|GetHeldObject) "ECC_Pawn" "ECR_Ignore")
      (Variables|Default|SetbIsHoldingObject true))))

(event Custom|HeldItemReset
  (if (Variables|Default|GetbIsHoldingObject)
    (Variables|Default|SetbIsHoldingObject false)))

(event EventBeginPlay
  (Variables|Default|SetMovementRegular (Variables|/Script/Engine.CharacterMovementComponent|GetMaxWalkSpeed (Variables|Character|GetCharacterMovement))))

(event Collision|EventActorBeginOverlap
  (params (OtherActor :type Actor%20Object%20Reference)))

(event EventTick
  (params (DeltaSeconds :type Float%20%28single-precision%29))
  (bind _firstpersoncameracomponent (Variables|Default|GetFirstPersonCameraComponent))
  (bind _heldobjectlocation (Variables|Default|GetHeldObjectLocation))
  ;[1 1 1] Update Location of Rotation of Held object
  (Class|PhysicsHandleComponent|SetTargetLocationandRotation (Variables|Default|GetPhysicsHandle) (Transformation|GetWorldLocation _heldobjectlocation) (Transformation|GetWorldRotation _heldobjectlocation))
  ;[1 1 1] Draw Teleport Parabola if ModeTeleport is true
  (if (Variables|Default|GetbModeTeleport)
    (CallFunction|GetTeleportLocationParabola (Transformation|GetWorldLocation _firstpersoncameracomponent) (Math|Vector|GetForwardVector _firstpersoncameracomponent) 10 0.1 1.5e+03)))

(event Input|MouseEvents|LeftMouseButton
  (params (Key :type Key%20Structure))
  (:Pressed
    (if (Variables|Default|GetbIsHoldingObject)
      (if (Utilities|DoesObjectImplementInterface (Variables|Default|GetHeldObjectActor) "/Game/Final_level/BPI_HeldAction.BPI_HeldAction_C")
        (bind _asbpi_held_action (Utilities|Casting|CastToBPI_HeldAction (Variables|Default|GetHeldObjectActor))
          (:then
            (Default|UseAction _asbpi_held_action))
          (:CastFailed
            (Development|PrintString "Failed Cast to BPI_HeldAction")))
        (else
          (Development|PrintString "NOT BPI_HeldAction")))
      (else
        (Development|PrintString "Not Holding Item")))))

(event Input|KeyboardEvents|E
  (params (Key :type Key%20Structure))
  ;[1 1 1] Input (E) - Pickup/Drop items and Teleport to Location
  (:Pressed
    (if (Variables|Default|GetbModeTeleport)
      (if (Variables|Default|GetbCanTeleport)
        (CallFunction|TeleporttoLocation (Variables|Default|GetTeleportLocation))
        (Development|PrintString "Teleport Location Acceptable"))
      (elif (Variables|Default|GetbIsHoldingObject)
        (CallFunction|DropObject)
        (else
          (CallFunction|AttemptInteract))))))

(event Input|KeyboardEvents|T
  (params (Key :type Key%20Structure))
  ;[1 1 1] Press T to Toggle Point and Click Teleport
  (:Pressed
    (CallFunction|ToggleTeleportMode)
    (CallFunction|DropObject)))

(event Input|KeyboardEvents|E
  (params (Key :type Key%20Structure))
  ;[1 1 1] Press E to attempt to interact with object in front of you
)

(event Input|KeyboardEvents|Q
  (params (Key :type Key%20Structure))
  (bind _heldobject (Variables|Default|GetHeldObject))
  (:Pressed
    (if (Variables|Default|GetbIsHoldingObject)
      (Utilities|IsValid (Variables|Default|GetHeldObjectActor)
        (:Is%20Valid
          (CallFunction|DropObject)
          (Physics|AddImpulseatLocation _heldobject (* (Math|Vector|GetForwardVector (Variables|Default|GetFirstPersonCameraComponent)) 6e+04) (Transformation|GetWorldLocation _heldobject) "None")))
      (else
        (Development|PrintString "Not Holding Item")))))

(event Input|KeyboardEvents|Q
  (params (Key :type Key%20Structure)))

(event Input|KeyboardEvents|LeftShift
  (params (Key :type Key%20Structure))
  (:Pressed
    (Variables|/Script/Engine.CharacterMovementComponent|SetMaxWalkSpeed (Variables|Character|GetCharacterMovement) (Variables|Default|GetMovementSprint)))
  (:Released
    (Variables|/Script/Engine.CharacterMovementComponent|SetMaxWalkSpeed (Variables|Character|GetCharacterMovement) (Variables|Default|GetMovementRegular))))

(fn ConstructionScript)

(fn TeleporttoLocation
  (params (Location :type Vector))
  (Transformation|SetActorLocation (Math|Vector|MakeVector (.x Location) (.y Location) (+ (.z Location) (Variables|/Script/Engine.CapsuleComponent|GetCapsuleHalfHeight (Variables|Default|GetCapsuleComponent)))) false false))

(fn GetTeleportLocationParabola
  (params (Location :type Vector) (Forward :type Vector) (Steps :type Integer) (TimeStep :type Float%20%28single-precision%29) (Speed :type Float%20%28single-precision%29))
  (Utilities|FlowControl|Sequence
    (:then_0
      (bind _output_get (LocalVariables|SetInitialLocation Location))
      (LocalVariables|SetPreviousLocation _output_get)
      (LocalVariables|SetVelocity (* Forward Speed))
      (LocalVariables|SetTime TimeStep))
    (:then_1
      (bind _index (Utilities|FlowControl|ForLoopwithBreak 1 Steps :!label _label)
        (:LoopBody
          ;[1 1 1] missing interactive, teleport
          (bind (_outhit _returnvalue) (Collision|LineTraceByChannel (LocalVariables|GetPreviousLocation) (+ (Math|Vector|MakeVector (* (.X (Math|Vector|BreakVector (LocalVariables|GetVelocity))) (* _index (LocalVariables|GetTime))) (* (.Y (Math|Vector|BreakVector (LocalVariables|GetVelocity))) (* _index (LocalVariables|GetTime))) (- (* (.Z (Math|Vector|BreakVector (LocalVariables|GetVelocity))) (* _index (LocalVariables|GetTime))) (* (* _index (LocalVariables|GetTime)) (* _index (LocalVariables|GetTime)) 0.5 2e+03))) (LocalVariables|GetInitialLocation)) "TraceTypeQuery3" false 0 "ForOneFrame" true "(R=1.000000,G=0.009645,B=0.000000,A=1.000000)"))
          (LocalVariables|SetPreviousLocation (+ (Math|Vector|MakeVector (* (.X (Math|Vector|BreakVector (LocalVariables|GetVelocity))) (* _index (LocalVariables|GetTime))) (* (.Y (Math|Vector|BreakVector (LocalVariables|GetVelocity))) (* _index (LocalVariables|GetTime))) (- (* (.Z (Math|Vector|BreakVector (LocalVariables|GetVelocity))) (* _index (LocalVariables|GetTime))) (* (* _index (LocalVariables|GetTime)) (* _index (LocalVariables|GetTime)) 0.5 2e+03))) (LocalVariables|GetInitialLocation)))
          (if _returnvalue
            (Utilities|FlowControl|Sequence
              (:then_0
                (goto _label Break))
              (:then_1
                (if (> (Math|Vector|DotProduct (.Normal (Collision|BreakHitResult _outhit)) "0, 0,1.000000") 0.1)
                  (bind _output_get_2 (Variables|Default|SetbCanTeleport (> (Math|Vector|DotProduct (.Normal (Collision|BreakHitResult _outhit)) "0, 0,1.000000") 0.1)))
                  (if _output_get_2
                    (bind _output_get_3 (Variables|Default|SetTeleportLocation (.Location (Collision|BreakHitResult _outhit))))
                    (Class|KismetSystemLibrary|DrawDebugCylinder _output_get_3 (+ _output_get_3 (* (.Normal (Collision|BreakHitResult _outhit)) 1e+01)) 3e+01 25 "(R=0.000000,G=0.542093,B=1.000000,A=1.000000)" 0.0 1.0)))))
            (else
              (Variables|Default|SetbCanTeleport false))))))))

(fn ToggleTeleportMode
  (if (Variables|Default|GetbModeTeleport)
    (Development|PrintString "ModeTeleport: OFF")
    (Variables|Default|SetbModeTeleport false)
    (else
      (Development|PrintString "ModeTeleport: ON")
      (Variables|Default|SetbModeTeleport true))))