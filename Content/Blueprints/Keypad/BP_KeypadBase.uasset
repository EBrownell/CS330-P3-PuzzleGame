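; Keypad actor that collects button presses and opens a linked door when the entered code matches.
; RecieveButton appends each key to an input string, clears it when it grows longer than the code, and shows it on a text display.
; The expected code and its length come from a CodeGenny reference, and a full match calls Open on MyControlledDoor.
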(event EventBeginPlay
  (Rendering|Components|TextRender|SetText (Variables|Default|GetDisplay) (Utilities|Text|ToText(String) (Variables|Default|Getinput))))

(event Collision|EventActorBeginOverlap
  (params (OtherActor :type Actor%20Object%20Reference)))

(event EventTick
  (params (DeltaSeconds :type Float%20%28single-precision%29)))

(fn ConstructionScript)

(fn RecieveButton
  (params (inputKey :type Integer))
  (bind _output_get (Variables|Default|Setinput (Utilities|String|Append (Variables|Default|Getinput) (Utilities|String|ToString(Integer) inputKey))))
  (bind _returnvalue (Class|CipherGenner|GetCodeLen (Variables|Default|GetCodeGenny)))
  (if (> (Utilities|String|Len _output_get) _returnvalue)
    (Variables|Default|Setinput ""))
  (Rendering|Components|TextRender|SetText (Variables|Default|GetDisplay) (Utilities|Text|ToText(String) (Variables|Default|Getinput)))
  (bind _returnvalue_2 (Class|CipherGenner|GetCode (Variables|Default|GetCodeGenny)))
  (if (Utilities|Enum|Equal(Enum) (Variables|Default|Getinput) _returnvalue_2)
    (Default|Open (Variables|Default|GetMyControlledDoor))))