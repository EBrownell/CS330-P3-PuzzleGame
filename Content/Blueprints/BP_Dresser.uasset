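; BP_Dresser is an interactable dresser with a drawer that can hold a key for a linked BP_Door.
; Interact toggles the drawer through the Drawer timeline, which slides Cube1 along X, with IsMoving blocking re-triggers mid-motion.
; Interacting with an open drawer that contains the key clears the key, sets the TextRender height and opens the door instead of closing the drawer.
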(event EventBeginPlay)

(event Collision|EventActorBeginOverlap
  (params (OtherActor :type Actor%20Object%20Reference)))

(event EventTick
  (params (DeltaSeconds :type Float%20%28single-precision%29)))

(event EventInteract
  (bind _textrender (Variables|Default|GetTextRender))
  (bind _cube1 (Variables|Default|GetCube1))
  (bind _relativelocation (Variables|/Script/Engine.SceneComponent|GetRelativeLocation _textrender))
  (bind _relativelocation_2 (Variables|/Script/Engine.SceneComponent|GetRelativeLocation _cube1))
  (if (not (Variables|Default|Getis_moving))
    (Variables|Default|Setis_moving true)
    (if (Variables|Default|Getis%20open)
      (if (Variables|Default|GetContains_Key)
        ;[1 1 1] Early Key
        (Variables|Default|SetContains_Key false)
        (bind _asbp_door (Utilities|Casting|CastToBP_Door (Variables|Default|GetDoor)))
        (Transformation|SetRelativeLocation _textrender (Math|Vector|MakeVector (.x _relativelocation) (.y _relativelocation) 45.0) false false)
        (Variables|Default|Setis_moving false)
        (Default|Open _asbp_door)
        (else
          (bind _newtrack_0 (Timeline|drawer ReverseFromEnd)
            (:Update
              (Transformation|SetRelativeLocation (Variables|Default|GetCube1) (Math|Vector|MakeVector (.x _newtrack_0) (.y _relativelocation_2) (.z _relativelocation_2)) false false))
            (:Finished
              (Variables|Default|Setis_moving false)
              (if (Variables|Default|Getis%20open)
                (Variables|Default|Setis%20open false)
                (else
                  (Variables|Default|Setis%20open true)))))))
      (else
        (Timeline|drawer PlayFromStart)))))

(fn ConstructionScript)