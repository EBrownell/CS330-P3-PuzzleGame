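; Sliding door Blueprint that toggles open and closed on Interact, with a sound.
; The DoorOpen timeline plays or reverses to move the mesh along its relative Y axis, flipping IsOpen when finished.
; CanOpen gates interaction: it clears during movement, is set by Open, and Interact prints a message while it is false.
; LockDoor sets IsLocked, which silently blocks Interact and is never cleared here.
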(event Custom|Open
  (Variables|Default|SetCan%20Open true))

(event Custom|LockDoor
  (Variables|Default|SetisLocked true))

(event EventBeginPlay)

(event Collision|EventActorBeginOverlap
  (params (OtherActor :type Actor%20Object%20Reference)))

(event EventTick
  (params (DeltaSeconds :type Float%20%28single-precision%29)))

(event EventInteract
  (bind _mesh (Variables|Default|GetMesh))
  (bind _relativelocation (Variables|/Script/Engine.SceneComponent|GetRelativeLocation _mesh))
  (if (not (Variables|Default|GetisLocked))
    (if (Variables|Default|GetCan%20Open)
      (Audio|PlaySoundatLocation (Variables|Default|GetAudio%20Cue) (Transformation|GetWorldLocation (Variables|Default|GetMesh)) "0, 0, 0" (Variables|Default|GetAudio%20Volume%20Multiplier) (Variables|Default|GetAudio%20Pitch%20Multiplier) 0.0 0 0 0)
      (if (Variables|Default|GetisOpen)
        (bind _newtrack_3 (Timeline|Door%20Open ReverseFromEnd)
          (:Update
            (Transformation|SetRelativeLocation _mesh (Math|Vector|MakeVector (.x _relativelocation) _newtrack_3 (.z _relativelocation)) false false)
            (Variables|Default|SetCan%20Open false))
          (:Finished
            (Variables|Default|SetCan%20Open true)
            (if (Variables|Default|GetisOpen)
              (Variables|Default|SetisOpen false)
              (else
                (Variables|Default|SetisOpen true)))))
        (else
          (Timeline|Door%20Open Play)))
      (else
        (Development|PrintString (Variables|Default|GetMessage))))))

(fn ConstructionScript)