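; Dresser is an interactable Blueprint with a drawer that slides open and closed.
; Interact plays the Drawer timeline forward or in reverse based on IsOpen, and its track drives only the X relative location of Cube1.
; IsMoving ignores interactions during the slide, and the timeline's finish clears it and toggles IsOpen.
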(event EventBeginPlay)

(event Collision|EventActorBeginOverlap
  (params (OtherActor :type Actor%20Object%20Reference)))

(event EventTick
  (params (DeltaSeconds :type Float%20%28single-precision%29)))

(event EventInteract
  (bind _cube1 (Variables|Default|GetCube1))
  (bind _relativelocation (Variables|/Script/Engine.SceneComponent|GetRelativeLocation _cube1))
  (if (not (Variables|Default|Getis_moving))
    (Variables|Default|Setis_moving true)
    (if (Variables|Default|Getis%20open)
      (bind _newtrack_0 (Timeline|drawer ReverseFromEnd)
        (:Update
          (Transformation|SetRelativeLocation (Variables|Default|GetCube1) (Math|Vector|MakeVector (.x _newtrack_0) (.y _relativelocation) (.z _relativelocation)) false false))
        (:Finished
          (Variables|Default|Setis_moving false)
          (if (Variables|Default|Getis%20open)
            (Variables|Default|Setis%20open false)
            (else
              (Variables|Default|Setis%20open true)))))
      (else
        (Timeline|drawer PlayFromStart)))))

(fn ConstructionScript)