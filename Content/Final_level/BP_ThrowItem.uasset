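; BP_ThrowItem is a throwable item actor that damages enemies it hits.
; Its Hit event applies Damage to a living BP_Enemy, prints a debug message, then briefly disables CanDamage to prevent rapid repeat hits.
; Two custom events switch the static mesh's response to the Pawn channel between Ignore and Block, toggling collision with the player and other pawns.
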(event OnComponentHit(StaticMesh)
  (params (HitComponent :type Primitive%20Component%20Object%20Reference) (OtherActor :type Actor%20Object%20Reference) (OtherComp :type Primitive%20Component%20Object%20Reference) (NormalImpulse :type Vector :default "0, 0, 0") (Hit :type Hit%20Result%20Structure%20%28by%20ref%29)))

(event EventBeginPlay)

(event Collision|EventActorBeginOverlap
  (params (OtherActor :type Actor%20Object%20Reference)))

(event EventTick
  (params (DeltaSeconds :type Float%20%28single-precision%29)))

(event EventRemovePlayerCollision
  (Collision|SetCollisionResponsetoChannel (Variables|Default|GetStaticMesh) "ECC_Pawn" "ECR_Ignore"))

(event EventAddPlayerCollision
  (Collision|SetCollisionResponsetoChannel (Variables|Default|GetStaticMesh) "ECC_Pawn" "ECR_Block"))

(event Collision|EventHit
  (params (MyComp :type Primitive%20Component%20Object%20Reference) (Other :type Actor%20Object%20Reference) (OtherComp :type Primitive%20Component%20Object%20Reference) (bSelfMoved :type Boolean) (HitLocation :type Vector :default "0, 0, 0") (HitNormal :type Vector :default "0, 0, 0") (NormalImpulse :type Vector :default "0, 0, 0") (Hit :type Hit%20Result%20Structure%20%28by%20ref%29))
  (if (Variables|Default|GetCanDamage)
    (bind _asbp_enemy (Utilities|Casting|CastToBP_Enemy Other))
    (if (not (Variables|/Game/Final_level/BP_Enemy.BP_Enemy_C|GetbIsDead _asbp_enemy))
      (Game|Damage|ApplyDamage _asbp_enemy (Variables|Default|GetDamage) 0 0)
      (Development|PrintString "I Hit something (new)")
      (Variables|Default|SetCanDamage false)
      (Utilities|FlowControl|Delay 0.1)
      (Variables|Default|SetCanDamage true))))

(fn ConstructionScript)