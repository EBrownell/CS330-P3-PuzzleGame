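; BP_Enemy is an enemy character whose defeat opens the WinScreen level.
; Once turned on, it wanders between random navmesh points and, after a short delay, fires BP_EnemyProjectile at the player on a self-rescheduling, randomly timed timer.
; AnyDamage lowers health and raises walk speed in proportion to damage, or on death stops attacks and shows "Fainted".
; Tick updates the health bar and turns widget and text toward the player.
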(event OnComponentHit(CapsuleComponent)
  (params (HitComponent :type Primitive%20Component%20Object%20Reference) (OtherActor :type Actor%20Object%20Reference) (OtherComp :type Primitive%20Component%20Object%20Reference) (NormalImpulse :type Vector :default "0, 0, 0") (Hit :type Hit%20Result%20Structure%20%28by%20ref%29)))

(event Custom|DieAnywhereElse
  (AI|AIMoveTo self (.RandomLocation (Class|NavigationSystemV1|GetRandomPointinNavigableRadius (Transformation|GetActorLocation) 4e+02 (Variables|Default|GetNavMesh) 0)) 0 5.0 false
    (:OnSuccess
      _)
    (:OnFail
      _))
  (if (not (Variables|Default|GetbIsDead))
    (CallFunction|DieAnywhereElse)))

(event Custom|TakeDamage
  (params (dmg_taken :type Float%20%28single-precision%29)))

(event Custom|UpdateHealthDisplay
  (if (Variables|Default|GetbIsDead)
    (Rendering|Components|TextRender|SetText (Variables|Default|GetTextRender) (Utilities|Text|FormatText "Fainted"))
    (else
      (Rendering|Components|TextRender|SetText (Variables|Default|GetTextRender) (Utilities|Text|ToText(String) (Utilities|String|Append (Utilities|String|ToString(Float) (Variables|Default|GetHealthCurrent)) "/" (Utilities|String|ToString(Float) (Variables|Default|GetHealthMax))))))))

(event Custom|TurnOn
  (Variables|Default|SetbIsActive true)
  (CallFunction|DieAnywhereElse)
  (Utilities|FlowControl|Delay 2.0)
  (CallFunction|Attack))

(event Custom|Attack
  (bind _returnvalue (Transformation|GetActorLocation))
  (bind _returnvalue_2 (Game|GetPlayerCharacter 0))
  (bind _returnvalue_3 (Transformation|GetActorLocation _returnvalue_2))
  (bind _returnvalue_4 (+ _returnvalue "0, 0,100.000000"))
  (bind _returnvalue_5 (- _returnvalue_3 _returnvalue_4))
  (bind _returnvalue_6 (Math|Vector|Normalize _returnvalue_5))
  (if (not (Variables|Default|GetbIsDead))
    (bind _returnvalue_7 (Game|SpawnActorfromClass "/Game/Final_level/BP_EnemyProjectile.BP_EnemyProjectile_C" (Math|Transform|MakeTransform (+ _returnvalue_4 (* _returnvalue_6 6e+01)) (Math|Rotator|FindLookatRotation _returnvalue_4 _returnvalue_3) "1,1,1") "Undefined" 0 0))
    (Physics|SetPhysicsLinearVelocity (Variables|/Game/Final_level/BP_EnemyProjectile.BP_EnemyProjectile_C|GetStaticMesh _returnvalue_7) (* _returnvalue_6 8e+02) false "None")
    (AddComponent|AddRotatingMovementComponent _returnvalue_7)
    (bind _returnvalue_8 (Utilities|Time|SetTimerbyFunctionName 0 "Attack" (Math|Random|RandomFloatinRange 1.0 3.0)))
    (Variables|Default|SetAttackTimeHandle _returnvalue_8)))

(event Custom|FacePlayer_Widget
  (Transformation|SetWorldRotation (Variables|Default|GetWidget) (Math|Rotator|FindLookatRotation (Transformation|GetActorLocation) (Transformation|GetActorLocation (Game|GetPlayerCharacter 0))) false false))

(event Custom|FacePlayer_Text
  (Transformation|SetWorldRotation (Variables|Default|GetTextRender) (Math|Rotator|FindLookatRotation (Transformation|GetActorLocation) (Transformation|GetActorLocation (Game|GetPlayerCharacter 0))) false false))

(event EventBeginPlay
  (Variables|Default|SetHealthCurrent (Variables|Default|GetHealthMax)))

(event Collision|EventActorBeginOverlap
  (params (OtherActor :type Actor%20Object%20Reference)))

(event EventTick
  (params (DeltaSeconds :type Float%20%28single-precision%29))
  (CallFunction|UpdateEnemyHPBar)
  (CallFunction|FacePlayerWidget)
  (CallFunction|FacePlayerText))

(event Game|Damage|EventAnyDamage
  (params (Damage :type Float%20%28single-precision%29) (DamageType :type Damage%20Type%20Object%20Reference) (InstigatedBy :type Controller%20Object%20Reference) (DamageCauser :type Actor%20Object%20Reference))
  (Variables|Default|SetHealthCurrent (- (Variables|Default|GetHealthCurrent) Damage))
  (if (<= (Variables|Default|GetHealthCurrent) 0.0)
    (Variables|Default|SetHealthCurrent 0.0)
    (Variables|Default|SetbIsDead true)
    (Variables|Actor|SetbCanBeDamaged false)
    (Components|Movement|StopMovementImmediately (Variables|Character|GetCharacterMovement))
    (Utilities|Time|ClearandInvalidateTimerbyHandle (Variables|Default|GetAttackTimeHandle))
    (else
      (Variables|/Script/Engine.CharacterMovementComponent|SetMaxWalkSpeed (Variables|Character|GetCharacterMovement) (+ (Class|MovementComponent|GetMaxSpeed (Variables|Character|GetCharacterMovement)) (* Damage 3.0)))))
  (CallFunction|UpdateHealthDisplay)
  (if (<= (Variables|Default|GetHealthCurrent) 0.0)
    (Utilities|FlowControl|Delay 2.0)
    (Game|OpenLevel(byName) "WinScreen")))

(fn ConstructionScript)

(fn UpdateEnemyHPBar
  (bind _asenemy_umg (Utilities|Casting|CastToEnemyUMG (UserInterface|GetUserWidgetObject (Variables|Default|GetWidget))))
  (Progress|SetPercent (Variables|/Game/Final_level/EnemyUMG.EnemyUMG_C|GetProgressBar_39 _asenemy_umg) (/ (Variables|Default|GetHealthCurrent) (Variables|Default|GetHealthMax))))