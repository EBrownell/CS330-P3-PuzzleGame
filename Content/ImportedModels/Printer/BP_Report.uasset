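; BP_Report is an interactable report pickup that unlocks a door when used.
; Other Blueprints hand it a door reference through GrabDoorPtr and toggle its availability through Set_isInteractable.
; On Interact, if interactable, it casts the stored reference to BP_Door, calls Open and destroys itself.
; Debug prints mark success and the cast or validity failures.
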(event Custom|GrabDoorPtr
  (params (NewParam :type Actor%20Object%20Reference))
  (Variables|Default|SetDoor NewParam))

(event Custom|Set_isInteractable
  (params (NewParam :type Boolean))
  (Variables|Default|SetbIsInteractable NewParam))

(event EventBeginPlay)

(event Collision|EventActorBeginOverlap
  (params (OtherActor :type Actor%20Object%20Reference)))

(event EventTick
  (params (DeltaSeconds :type Float%20%28single-precision%29)))

(event EventInteract
  (bind _door (Variables|Default|GetDoor))
  (if (Variables|Default|GetbIsInteractable)
    (Development|PrintString "Interacting with Report")
    (bind _asbp_door (Utilities|Casting|CastToBP_Door _door)
      (:then
        (Utilities|IsValid _door
          (:Is%20Valid
            (Default|Open _asbp_door)
            (Development|PrintString "Door Unlocked")
            (Actor|DestroyActor))
          (:Is%20Not%20Valid
            (Development|PrintString "Failed isValid"))))
      (:CastFailed
        (Development|PrintString "Failed Cast")))))

(fn ConstructionScript)