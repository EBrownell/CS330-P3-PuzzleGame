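; Interactable puzzle printer that needs paper and ink before it can print a single report linked to a door.
; A box overlap consumes BP_Paper or BP_Ink, resets the player's held item and marks the printer fixed once both are in.
; Interact prints debug hints or spawns BP_Report, passing it the Door reference.
; A timeline slides the report along X by adding to its current location, then makes it interactable.
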(event OnComponentBeginOverlap(Box)
  (params (OverlappedComponent :type Primitive%20Component%20Object%20Reference) (OtherActor :type Actor%20Object%20Reference) (OtherComp :type Primitive%20Component%20Object%20Reference) (OtherBodyIndex :type Integer) (bFromSweep :type Boolean) (SweepResult :type Hit%20Result%20Structure%20%28by%20ref%29))
  (bind _returnvalue (Game|Player|GetPlayerPawn 0))
  ;[1 1 1] Paper or Ink is given to printer
  (bind _asbp_paper (Utilities|Casting|CastToBP_Paper OtherActor)
    (:then
      (Utilities|IsValid _asbp_paper
        (:Is%20Valid
          (Actor|DestroyActor _asbp_paper)
          (bind _asbp_player_character (Utilities|Casting|CastToBP_PlayerCharacter _returnvalue))
          (Default|HeldItemReset _asbp_player_character)
          (Development|PrintString "Printer got Paper")
          (Variables|Default|SetbHasPaper true)
          (CallFunction|UpdateIsFixed))))
    (:CastFailed
      (bind _asbp_ink (Utilities|Casting|CastToBP_Ink OtherActor))
      (Utilities|IsValid _asbp_ink
        (:Is%20Valid
          (Actor|DestroyActor _asbp_ink)
          (bind _asbp_player_character_2 (Utilities|Casting|CastToBP_PlayerCharacter _returnvalue))
          (Default|HeldItemReset _asbp_player_character_2)
          (Development|PrintString "Printer got Ink")
          (Variables|Default|SetbHasInk true)
          (CallFunction|UpdateIsFixed))))))

(event Custom|Update%20is%20Fixed
  ;[1 1 1] Check the state of isFixed
  (if (not (Variables|Default|GetbIsFixed))
    (if (Variables|Default|GetbHasPaper)
      (if (Variables|Default|GetbHasInk)
        (Variables|Default|SetbIsFixed true))
      (elif (Variables|Default|GetbHasInk)
        _))))

(event Custom|PrintPaper
  (bind _paperspawnpoint (Variables|Default|GetPaperSpawnPoint))
  (bind _returnvalue (Game|SpawnActorfromClass "/Game/ImportedModels/Printer/BP_Report.BP_Report_C" (Math|Transform|MakeTransform (Transformation|GetWorldLocation _paperspawnpoint) (Transformation|GetWorldRotation _paperspawnpoint) "1,1,1") "AlwaysSpawn" 0 0))
  (bind _output_get (Variables|Default|SetReport _returnvalue))
  (Variables|Default|SetbHasPrinted true)
  (bind _asbp_report (Utilities|Casting|CastToBP_Report _output_get)
    (:then
      (Default|GrabDoorPtr _asbp_report (Variables|Default|GetDoor))
      (bind _newtrack_0 (Timeline|Timeline_0 Play)
        (:Update
          (Transformation|SetActorRelativeLocation (Variables|Default|GetReport) (Math|Vector|MakeVector (+ (.x _newtrack_0) (.x (Transformation|GetActorLocation (Variables|Default|GetReport)))) (.y (Transformation|GetActorLocation (Variables|Default|GetReport))) (.z (Transformation|GetActorLocation (Variables|Default|GetReport))))))
        (:Finished
          (bind _asbp_report_2 (Utilities|Casting|CastToBP_Report (Variables|Default|GetReport)))
          (Default|SetIsInteractable _asbp_report_2 true)
          (Development|PrintString "Finished!!!!!"))))
    (:CastFailed
      (Development|PrintString "Failed Cast In Printer"))))

(event EventBeginPlay)

(event Collision|EventActorBeginOverlap
  (params (OtherActor :type Actor%20Object%20Reference)))

(event EventTick
  (params (DeltaSeconds :type Float%20%28single-precision%29)))

(event EventInteract
  (if (not (Variables|Default|GetbHasPrinted))
    (if (Variables|Default|GetbIsFixed)
      (Development|PrintString "Success")
      (CallFunction|PrintPaper)
      (elif (Variables|Default|GetbHasPaper)
        (if (not (Variables|Default|GetbHasInk))
          (Development|PrintString "Printer requires Ink"))
        (elif (Variables|Default|GetbHasInk)
          (Development|PrintString "Printer requires Paper")
          (else
            (Development|PrintString (Variables|Default|GetMessage))))))))

(fn ConstructionScript)