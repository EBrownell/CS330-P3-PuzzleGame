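; BP_ToyGun is a holdable nerf gun that fires foam darts when the player triggers its use action with left click.
; UseAction checks an ammo count filled at BeginPlay, then either prints an empty message or calls Shoot.
; Shoot spawns a BP_Dart ahead of the mesh with a pitch offset, launches it by setting physics velocity, and decrements ammo.
; Two events toggle the mesh's Pawn collision between Ignore and Block.
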(event Custom|Shoot
  (bind _staticmesh (Variables|Default|GetStaticMesh))
  (bind _returnvalue (Transformation|GetWorldTransform _staticmesh))
  (bind (_roll _pitch _yaw) (Math|Rotator|BreakRotator (.rotation _returnvalue)))
  ;[1 1 1] Fires a nerf gun bullet
  (bind _returnvalue_2 (Game|SpawnActorfromClass "/Game/ImportedModels/ToyGun/Ammo/BP_Dart.BP_Dart_C" (Math|Transform|MakeTransform (+ (* (Math|Vector|GetForwardVector _staticmesh) 26.0) (Math|Vector|MakeVector (.x (.location _returnvalue)) (.y (.location _returnvalue)) (+ (.z (.location _returnvalue)) 5.0))) (Math|Rotator|MakeRotator _roll (+ _pitch 9e+01) _yaw) "1,1,1") "Undefined" 0 0))
  (Class|PrimitiveComponent|SetAllPhysicsLinearVelocity (Variables|/Game/ImportedModels/ToyGun/Ammo/BP_Dart.BP_Dart_C|GetTube _returnvalue_2) (* (Math|Vector|GetForwardVector (Variables|Default|GetStaticMesh)) 1.5e+03) false)
  (Variables|Default|SetAmmoCurrent (- (Variables|Default|GetAmmoCurrent) 1)))

(event EventBeginPlay
  (Variables|Default|SetAmmoCurrent (Variables|Default|GetAmmoMax)))

(event Collision|EventActorBeginOverlap
  (params (OtherActor :type Actor%20Object%20Reference)))

(event EventTick
  (params (DeltaSeconds :type Float%20%28single-precision%29)))

(event EventUseAction
  ;[1 1 1] Action that is triggered when play has pressed appropriate button while holding this item (Left Click)
  (if (<= (Variables|Default|GetAmmoCurrent) 0)
    (Development|PrintString "Out of Ammo")
    (else
      (CallFunction|Shoot)
      (Development|PrintString "Bang"))))

(event EventRemovePlayerCollision
  (Collision|SetCollisionResponsetoChannel (Variables|Default|GetStaticMesh) "ECC_Pawn" "ECR_Ignore"))

(event EventAddPlayerCollision
  (Collision|SetCollisionResponsetoChannel (Variables|Default|GetStaticMesh) "ECC_Pawn" "ECR_Block"))

(fn ConstructionScript)